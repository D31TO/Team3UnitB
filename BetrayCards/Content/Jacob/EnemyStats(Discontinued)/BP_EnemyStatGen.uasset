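; Enemy stat generator that rolls and displays enemy health and AC for a round, scaled to the first player's TotalPlayerCards.
; Two seconds after BeginPlay it increments CurrentRound, rolls both stats within percentage bands, and derives hit damage from round, difficulty and player multipliers.
; It then starts that character's deliberation timer.
; The RPC events are empty stubs, and the multiplayer and random-number test chains are never run.
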(event `self.ReceiveBeginPlay`
  (`KismetSystemLibrary.Delay` 2.0)
  (`self.Generate Random Stats`))

(event `RPC_Client_DoSomething`
  ;[1 1 1] Jacob's Code
)

(event `Generate Random Stats`
  (`self.RoundIncrease`)
  (bind _asbp_top_down_character (cast `/Game/TopDown/Blueprints/BP_TopDownCharacter` (`GameplayStatics.GetPlayerCharacter` 0)))
  (bind _totalplayercards (`/Game/TopDown/Blueprints/BP_TopDownCharacter.TotalPlayerCards` _asbp_top_down_character))
  ;[0.3091 0.3049 1] Enemy Health
  (`KismetSystemLibrary.PrintString` (`KismetStringLibrary.Conv_IntToString` _totalplayercards) true true (struct :`R` 0.955806 :`G` 1.0 :`B` 0.966854 :`A` 1.0) 30.0) ; #players
  (bind _returnvalue (/ _totalplayercards 100))
  (bind _returnvalue_2 (`KismetMathLibrary.RandomIntegerInRange` (* _returnvalue 25) (* _returnvalue 45)))
  (bind _output_get (set `self.RdmEnemyHealth` _returnvalue_2))
  (`TextRenderComponent.K2_SetText` (`self.Enemy Health`) (`|FormatText` "Enemy Health: {int}" _output_get))
  ;[1 0.1249 0.1349] Enemy AC
  (bind _output_get_2 (set `self.SoldierTotal` (* (/ _returnvalue_2 100) 60)))
  (`TextRenderComponent.K2_SetText` (`self.Enemy AC`) (`|FormatText` "Enemy AC: {int}" _output_get_2))
  ;[1 0.8022 0] Sets Enemy Hit Damage
  (set `self.EnemyHitDamage` (* (+ (* (`self.CurrentRound`) (`self.DifficultyMultiplier`)) (`self.BaseEnemyDamage`)) (`self.PlayerMultiplier`)))
  ;[0 1 0.06679] Round Start System
  (`/Game/TopDown/Blueprints/BP_TopDownCharacter.BeginDeliberationTimer` _asbp_top_down_character 0))

(event `RPC_Server_DoSomething`
  ;[1 1 1] Jacob's Code
)

(event `RPC GenRndNum`
  ;[1 1 1] Jacob's Code
)

(event `RPC MultiCastPrintNum`
  ;[1 1 1] Jacob's Code
)

(fn `OnRep_Player Index`)

(fn `OnRep_RndNum`)

(fn `RoundIncrease`
  (`/Engine/EditorBlueprintResources/StandardMacros.IncrementInt` (`self.CurrentRound`)
    (:`  `
      (return))))

(fn `UserConstructionScript`)