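; Enemy stat generator that rolls an enemy's health, required soldiers and hit damage for each new round.
; After a short delay, it increments the round in PrimGameInstance and rolls health as a percentage of EveryCharactersCard.
; Soldier total derives from health, while damage scales with round, difficulty and player multiplier, and all three print as debug text.
; The RPC events and OnRep functions are empty stubs, and the networking test code is disconnected.
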(event `/Game/Jacob/BPI_GenerateEnemies.BeginEnemyGeneration`
  (`KismetSystemLibrary.Delay` 3.0)
  (`self.Generate Random Stats`))

(event `RPC_Client_DoSomething`
  ;[1 1 1] Jacob's Code
)

(event `Generate Random Stats`
  (`self.RoundIncrease`)
  (bind _asprim_game_instance (cast `/Game/GameInstance/PrimGameInstance` (`GameplayStatics.GetGameInstance`)))
  (bind _returnvalue (/ (`/Game/GameInstance/PrimGameInstance.Every characters card` _asprim_game_instance) 100.0))
  ;[0.3091 0.3049 1] Enemy Health
  (bind _output_get (set `self.RdmEnemyHealth` (`KismetMathLibrary.FTrunc` (`KismetMathLibrary.RandomFloatInRange` (* _returnvalue 25.0) (* _returnvalue 45.0)))))
  (bind _output_get_2 (set `self.Enemy Health float` (`KismetMathLibrary.Conv_IntToDouble` _output_get)))
  ;[1 0.1249 0.1349] Enemy AC
  (bind _output_get_3 (set `self.SoldierTotal` (`KismetMathLibrary.FTrunc` (* (/ _output_get_2 100.0) 60.0))))
  ;[1 0.8022 0] Sets Enemy Hit Damage
  (bind _output_get_4 (set `self.EnemyHitDamage` (* (+ (* (`/Game/GameInstance/PrimGameInstance.CurrentRound` _asprim_game_instance) (`self.DifficultyMultiplier`)) (`self.BaseEnemyDamage`)) (`self.PlayerMultiplier`))))
  (`KismetSystemLibrary.PrintString` (`KismetTextLibrary.Conv_TextToString` (`|FormatText` "enemy health: {0}  \nSoldiers needed: {1} \nEnemy Hit Damage: {2}" _output_get_2 _output_get_3 _output_get_4)) true true (struct :`R` 1.0 :`G` 0.391573 :`A` 1.0) 30.0))

(event `RPC_Server_DoSomething`
  ;[1 1 1] Jacob's Code
)

(event `RPC GenRndNum`
  ;[1 1 1] Jacob's Code
)

(event `RPC MultiCastPrintNum`
  ;[1 1 1] Jacob's Code
)

(fn `OnRep_Player Index`)

(fn `OnRep_RndNum`)

(fn `RoundIncrease`
  (returns (CurrentRound :type Integer))
  (bind _asprim_game_instance (cast `/Game/GameInstance/PrimGameInstance` (`GameplayStatics.GetGameInstance`)))
  (bind _result (`/Engine/EditorBlueprintResources/StandardMacros.IncrementInt` (`/Game/GameInstance/PrimGameInstance.CurrentRound` _asprim_game_instance))
    (:`  `
      (return _result))))

(fn `UserConstructionScript`)