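; Game state that sets up a four-player card game and hands off to battle.
; On authority, PlayerJoined assigns a Joker, builds shuffled suited character, soldier and action decks (action data from a DataTable), and deals to each player controller.
; Leftover soldier and action cards form one shuffled deck saved in the GameInstance, which also receives a party health call.
; BattleDeck then reloads that deck, spawns each player's cards and triggers BP_BattleDeck.
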(event `test`
  ;[0 0.08854 0.02527] Core gameplay loops
  ;;[0 1 0.1167] Runs at the start of the game and makes the decks (Ran once)
)

(event `Serverside are cards played`
  (if (== (`self.TimesPlayed`) 4)
    (set `self.Major is done` true)))

(event `RPC Client Provide Character Card`
  (params (`Target Card` :type "/Game/Jack/CardMechanics/F_CharacterCardData Structure (by ref)") (`Target Player` :type "PlayerController Object Reference (by ref)"))
  ;[1 1 1] OLD CODE
  ;;[1 1 1] Only the target client will be given the target card (OLD)
  (`KismetSystemLibrary.PrintString` (`KismetSystemLibrary.GetClassDisplayName` (`.Object_11_EF3800814A6FC0EE8879E483F13A9F1F` (break `/Game/Jack/CardMechanics/F_CharacterCardData` `Target Card`))) true true (struct :`G` 0.66 :`B` 1.0 :`A` 1.0) 80.0))

(event `Battle Deck`
  ;[1 1 1] Battle Deck code
  ;;[1 1 1] Battle Deck code?
  (`self.Card deck Getter`)
  (for _index (range (`GameplayStatics.GetNumPlayerStates`))
    (bind _asbp_top_down_controller (cast `/Game/TopDown/Blueprints/BP_TopDownController` (`GameplayStatics.GetPlayerController` _index)))
    ;;;[0.1875 0 0.009669] Always needs the getter
    (`/Game/TopDown/Blueprints/BP_TopDownController.Player info Getter` _asbp_top_down_controller)
    (`/Game/TopDown/Blueprints/BP_TopDownController.In Battle Spawner` _asbp_top_down_controller)
    (`/Game/TopDown/Blueprints/BP_TopDownController.Spawn all cards` _asbp_top_down_controller))
  (bind _returnvalue (`GameplayStatics.GetActorOfClass` "/Game/Jack/BP_BattleDeck.BP_BattleDeck_C"))
  (`/Game/Jack/BP_BattleDeck.TESTY` _returnvalue))

(event `self.ReceiveBeginPlay`)

(event `RPCtoserver`)

(event `/Game/Jack/BPI_CustomGameState.PlayerJoined`
  (params (Controller :type "PlayerController Object Reference (by ref)"))
  ;[1 1 1] Shall run at the begining of the game
  ;;[0.09351 0.4635 0] Runs the basic gameplay loop
  (`KismetSystemLibrary.Delay` 5.0)
  (`/Engine/EditorBlueprintResources/ActorMacros.Switch Has Authority`
    (:`Authority`
      (if (== (`KismetArrayLibrary.Array_Length` (`self.PlayerArray`)) 4)
        (`/Engine/EditorBlueprintResources/StandardMacros.DoOnce` false
          (:`Completed`
            (`self.Decided the joker`)
            (`self.CreateCharacterDeck`)
            (`self.Creates All Cards`)
            (`self.Combine Both Playable Decks`)
            (for _index (range (`GameplayStatics.GetNumPlayerStates`))
              (bind _asbp_top_down_controller (cast `/Game/TopDown/Blueprints/BP_TopDownController` (`GameplayStatics.GetPlayerController` _index) :!pure true))
              (`/Game/TopDown/Blueprints/BP_TopDownController.Gives Unique character card` _asbp_top_down_controller)
              (`/Game/TopDown/Blueprints/BP_TopDownController.Total cards` _asbp_top_down_controller)
              ;;;[0.25 0.01636 0] Always needs the Setter
              (`/Game/TopDown/Blueprints/BP_TopDownController.Player Info Setter` _asbp_top_down_controller))
            (bind _asprim_game_instance (cast `/Game/GameInstance/PrimGameInstance` (`GameplayStatics.GetGameInstance`)))
            (`/Game/GameInstance/PrimGameInstance.Whole party total health` _asprim_game_instance)
            (`self.Battle Deck`)))))))

(event `toclients`
  (bind _asprim_game_instance (cast `/Game/GameInstance/PrimGameInstance` (`GameplayStatics.GetGameInstance`))))

(event `CustomEvent`)

(event `Sets Action card values`
  (params (`Current Row on Table` :type Integer) (`Action card` :type "/Game/Jack/CardMechanics/SoldierCards/BP_GenericCardTemplate Class Reference"))
  ;[1 0.6804 0.202] Sets the action card values
  (bind _returnvalue (`|GetDataTableRow` "/Game/DataTables/DT_NewAbilityCard.DT_NewAbilityCard" (`KismetStringLibrary.Conv_StringToName` (`KismetTextLibrary.Conv_TextToString` (`|FormatText` "NewRow_{x}" `Current Row on Table`))))
    (:`then`
      (`KismetArrayLibrary.Array_Add` (`self.ActionCard Deck`) (make `/Game/Jack/CardMechanics/F_PlayableCardData` (break `/Game/Jack/CardMechanics/F_PlayableCardData` _returnvalue) (`.Descrption_29_8AD20E234B7FC6EC251016A0F97A26EC` (break `/Game/Jack/CardMechanics/F_PlayableCardData` _returnvalue)) `Action card` 1 true (`.CardImage_32_CF11A81144095B919BB855B2BE0808B9` (break `/Game/Jack/CardMechanics/F_PlayableCardData` _returnvalue)))))
    (:`RowNotFound`
      (`KismetSystemLibrary.PrintString` "row not found"))))

(event `Combine Both Playable Decks`
  ;[0.01474 0.03864 0.1823] Combines Both Playable Decks And Shuffles
  (`KismetArrayLibrary.Array_Append` (`self.WholeCard Deck`) (`self.ActionCard Deck`))
  (`KismetArrayLibrary.Array_Append` (`self.WholeCard Deck`) (`self.SoldierCard Deck`))
  (`KismetArrayLibrary.Array_Shuffle` (`self.WholeCard Deck`))
  (`self.Card deck setter`))

(event `Creates All Cards`
  ;[0 0.3378 1] Makes the soldier and action card decks
  (for _array_element (`self.AllBaseCards`)
    (bind (_card_type _name) (defaults `Object` _array_element))
    (switch `/Game/Jack/CardMechanics/S_CardType` _card_type
      (:`NewEnumerator0`
        (for _ (range 60)
          (`KismetArrayLibrary.Array_Add` (`self.SoldierCard Deck`) (make `/Game/Jack/CardMechanics/F_PlayableCardData` _name "" _array_element 1 false "/Game/ConceptArt/Cards/Soldier_card.Soldier_card"))))
      (:`NewEnumerator1`
        ;;[1 1 1] changed from 20 to 14 as can be used eaiser
        (for _index (range 14)
          (`self.Sets Action card values` (/ (+ _index 1) 2) _array_element)))))
  (`KismetArrayLibrary.Array_Shuffle` (`self.ActionCard Deck`))
  (for _index_2 (range (`GameplayStatics.GetNumPlayerStates`))
    (bind _returnvalue (`GameplayStatics.GetPlayerController` _index_2))
    (`self.RPC Server Remove Top Soldier Card` _returnvalue)
    (`self.RPC Server Remove Top Ability Card` _returnvalue)))

(event `Card deck Getter`
  ;[0.02578 0 0.3125] Gets the card deck
  (bind _asprim_game_instance (cast `/Game/GameInstance/PrimGameInstance` (`GameplayStatics.GetGameInstance`)))
  (set `self.WholeCard Deck` (`/Game/GameInstance/PrimGameInstance.Cards in the deck not used` _asprim_game_instance)))

(event `CreateCharacterDeck`
  ;[1 0.1189 0.4779] Creates the character deck
  (for _array_element (`self.Card Charcters`)
    (for _index (range 4)
      (`KismetArrayLibrary.Array_Add` (`self.Character Deck`) (make `/Game/Jack/CardMechanics/F_CharacterCardData` (defaults `Object` _array_element) (select `int` _index :`0` "Hearts" :`1` "Diamonds" :`2` "Clubs" :`3` "Spades") _array_element))))
  (`KismetArrayLibrary.Array_Shuffle` (`self.Character Deck`))
  ;;[0.1615 0.1615 0.1615] Will repeat for how many players there are
  (for _index_2 (range (`GameplayStatics.GetNumPlayerStates`))
    (set `self.Players Controller` _index_2)
    (`self.RPC Server Remove Top Charcter Card` (`GameplayStatics.GetPlayerController` _index_2))))

(event `Card deck setter`
  ;[0.03454 0 0.2292] Sets the card deck
  (bind _asprim_game_instance (cast `/Game/GameInstance/PrimGameInstance` (`GameplayStatics.GetGameInstance`)))
  (`/Game/GameInstance/PrimGameInstance.Saves Whole Game Deck` _asprim_game_instance (`self.WholeCard Deck`)))

(event `RPC Server Remove Top Charcter Card`
  (params (`Target Player to give cards To` :type "PlayerController Object Reference (by ref)"))
  (bind _character_deck (`self.Character Deck`))
  ;[1 0.1063 0.7132] Removes Top Character Card and gives to specfic player controller
  (`/Game/TopDown/Blueprints/BP_TopDownController.SetPlayerCharacter` (cast `/Game/TopDown/Blueprints/BP_TopDownController` `Target Player to give cards To` :!pure true) (`|GetArrayItem` _character_deck) (`self.Players Controller`))
  (`KismetArrayLibrary.Array_Remove` _character_deck))

(event `RPC Server Remove Top Soldier Card`
  (params (`Targeted Player` :type "PlayerController Object Reference"))
  (bind _soldiercard_deck (`self.SoldierCard Deck`))
  ;[0 0.5217 0.849] Sends the soldier cards to the specfic player controller
  (for _ (range 4)
    (`/Game/TopDown/Blueprints/BP_TopDownController.Card Receieved` (cast `/Game/TopDown/Blueprints/BP_TopDownController` `Targeted Player` :!pure true) (`|GetArrayItem` _soldiercard_deck))
    (`KismetArrayLibrary.Array_Remove` _soldiercard_deck)))

(event `Decided the joker`
  ;[1 0 0.2363] Pick 1 out of the Max number of players to give the joker to
  (`/Game/TopDown/Blueprints/BP_TopDownController.Player Got the Joker Card` (cast `/Game/TopDown/Blueprints/BP_TopDownController` (`GameplayStatics.GetPlayerController` (`KismetMathLibrary.RandomInteger` 3)) :!pure true) (`self.Joker Card`)))

(event `RPC Server Remove Top Ability Card`
  (params (`Targeted Player` :type "PlayerController Object Reference"))
  (bind _actioncard_deck (`self.ActionCard Deck`))
  ;[0 0.7408 1] Sends the ability card to the  specfic player controller
  (`/Game/TopDown/Blueprints/BP_TopDownController.Card Receieved` (cast `/Game/TopDown/Blueprints/BP_TopDownController` `Targeted Player` :!pure true) (`|GetArrayItem` _actioncard_deck))
  (`KismetArrayLibrary.Array_Remove` _actioncard_deck))

(fn `UserConstructionScript`)