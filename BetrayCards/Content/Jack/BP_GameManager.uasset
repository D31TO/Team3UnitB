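; BP_GameManager is a game manager that starts card setup once enough players have joined.
; After a short delay on BeginPlay, the server polls the player controller count every tick until at least four are present.
; It then tells the CardManager to create the character deck.
; Soldier and spell deck creation, deck combining and a waiting message exist but are disconnected.
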(event `self.ReceiveBeginPlay`
  (`KismetSystemLibrary.Delay` 0.5)
  (`/Engine/EditorBlueprintResources/ActorMacros.Switch Has Authority`
    (:`Authority`
      (if (>= (`GameplayStatics.GetNumPlayerControllers`) 4) :!label _label
        (`KismetSystemLibrary.PrintString` "Enough players")
        (`/Game/Jack/CardMechanics/BP_CardManager.CreateCharacterDeck` (`self.CardManager`))
        (else
          (`KismetSystemLibrary.DelayUntilNextTick`)
          (goto _label))))))

(fn `UserConstructionScript`)