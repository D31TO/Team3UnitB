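; BP_BattleDeck manages the shared spare card pile and enemy setup for card battle encounters.
; TESTY loads the unused deck from PrimGameInstance and pulls randomized health, soldier and damage stats from BP_EnemyStatGen.
; Givescard deals cards from the top of the pile to every player's controller, and Setstheunusedpile saves the remainder to the game instance.
; Win/loss reward and party damage logic exists but is disconnected from any event.
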(event `TESTY`
  ;[1 1 1] Played at the start of the battle deck
  ;;[0.3702 0.4144 1] Get all information deck and party info
  (bind _asprim_game_instance (cast `/Game/GameInstance/PrimGameInstance` (`GameplayStatics.GetGameInstance`)))
  (`/Game/GameInstance/PrimGameInstance.All cards` _asprim_game_instance)
  (set `self.Spare card pile` (`/Game/GameInstance/PrimGameInstance.Cards in the deck not used` _asprim_game_instance))
  ;;[0.2572 0.7246 1] Gets the enemy info
  (bind _returnvalue (`GameplayStatics.GetActorOfClass` "/Game/Jacob/BP_EnemyStatGen.BP_EnemyStatGen_C"))
  (`/Game/Jacob/BP_EnemyStatGen.Generate Random Stats` _returnvalue)
  (bind _rdmenemyhealth (`/Game/Jacob/BP_EnemyStatGen.RdmEnemyHealth` _returnvalue))
  (set `self.Enemy Health` _rdmenemyhealth)
  (bind _soldiertotal (`/Game/Jacob/BP_EnemyStatGen.SoldierTotal` _returnvalue))
  (set `self.Soldier Needed` _soldiertotal)
  (bind _enemyhitdamage (`/Game/Jacob/BP_EnemyStatGen.EnemyHitDamage` _returnvalue))
  (set `self.Enemy  Damage` _enemyhitdamage)
  (`KismetSystemLibrary.PrintString` (`KismetStringLibrary.Concat_StrStr` "Enemy is: " "Unknown" " There health is: " (`KismetStringLibrary.Conv_IntToString` _rdmenemyhealth) " There soldier total is: " (`KismetStringLibrary.Conv_IntToString` _soldiertotal) " There Damage is: " (`KismetStringLibrary.Conv_IntToString` _enemyhitdamage)) true true (struct :`R` 0.195287 :`G` 1.0 :`B` 0.17946 :`A` 1.0) 1000.0))

(event `Sets the unused pile`
  ;[1 1 1] Will save the rest of the pile to the Game instance
  (`/Game/GameInstance/PrimGameInstance.Saves Whole Game Deck` (stale `TESTY` _asprim_game_instance) (`self.Spare card pile`)))

(event `Gives card`
  (params (`Times need to repeat` :type Integer))
  (bind _spare_card_pile (`self.Spare card pile`))
  ;[1 0.7982 0.1085] This will give a card to the player
  (for _index (range (`GameplayStatics.GetNumPlayerStates`))
    (for _ (range 1 (+ `Times need to repeat` 1))
      (`/Game/TopDown/Blueprints/BP_TopDownController.Card Receieved` (cast `/Game/TopDown/Blueprints/BP_TopDownController` (`GameplayStatics.GetPlayerController` _index) :!pure true) (`|GetArrayItem` _spare_card_pile))
      (`KismetArrayLibrary.Array_Remove` _spare_card_pile))))

(fn `UserConstructionScript`)