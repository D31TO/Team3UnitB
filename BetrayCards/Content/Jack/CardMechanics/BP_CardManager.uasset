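; BP_CardManager builds and shuffles the card decks for a multiplayer card game with soldier and spell cards.
; Separate events fill the soldier deck in sets of four and the spell deck with two entries per spell, combine them into PlayableCards, and shuffle a given deck.
; An older event gives a shuffled character card to a local player.
; Character deck creation and the server deal RPC are empty stubs, with their former logic left disconnected.
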(event `RPC Server Remove Top Character Card`
  (params (`Card Deck` :type "Array of /Game/Jack/CardMechanics/F_CharacterCardData Structure") (`Target Player to Give Card To` :type "PlayerController Object Reference (by ref)"))
  ;[1 1 1] Server Removes topmost card and gives it to specific client controller
)

(event `CreateCharacterDeck`
  ;[0 1 0.2239] Makes the Deck for the Characters
)

(event `CreateSoldierDeck`
  ;[1 0.3142 0.08274] Create soldier Deck
  (for _ (range 10)
    (for _index (range 4)
      (`KismetArrayLibrary.Array_Add` (`self.PlayableSoldierCards`)))
    (`KismetSystemLibrary.PrintString` "done one set of soldiers"))
  (`KismetSystemLibrary.PrintString` "all cards"))

(event `GivesCharacterToPlayer`
  (params (Character :type "Array of /Game/Jack/CardMechanics/F_CharacterCardData Structure") (`Target Player Controller` :type "PlayerController Object Reference"))
  ;[0.2552 0.2552 0.2552] Old
  (if (`Controller.IsLocalPlayerController` `Target Player Controller`)
    ;;[1 1 1] Gives to the player
    (`KismetArrayLibrary.Array_Shuffle` Character)
    (message `/Game/Jack/Interfaces/BPI_CharacterCard.GivesCharacterCards` (`GameplayStatics.GetPlayerCharacter` (`PlayerState.PlayerId` (`Controller.PlayerState` `Target Player Controller`))) (`|GetArrayItem` Character) null)
    (`KismetArrayLibrary.Array_Remove` Character)))

(event `CombineBothDecks`
  ;[1 0.9449 0.01481] Combines both the decks
  (`KismetArrayLibrary.Array_Append` (`self.PlayableCards`) (`self.PlayableSpellCards`))
  (`KismetArrayLibrary.Array_Append` (`self.PlayableCards`) (`self.PlayableSoldierCards`)))

(event `ShuffleDeck`
  (params (Card :type "Array of /Game/Jack/CardMechanics/F_PlayableCardData Structure"))
  ;[0 1 0.9281] Shuffles the card decks
  (`KismetArrayLibrary.Array_Shuffle` Card))

(event `CreateSpellCards`
  ;[0.3833 1 0.8388] Creates Spell Deck
  (for _ (`self.SpellCards`)
    ;;[1 1 1] Needs Good/Bad card
    (for _index (range 2)
      (`KismetArrayLibrary.Array_Add` (`self.PlayableSpellCards`)))))

(fn `OnRep_CharacterDeck`)

(fn `UserConstructionScript`)