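; Game State Blueprint that decides a round's outcome in a multiplayer game pitting good players against a Joker.
; On RoundEnd the server scans PlayerArray for dead players: a dead Joker means the good side wins, and three dead good players mean the Joker wins.
; Either win server-travels to Lobby2; otherwise NextRound resets the death count and reloads MazeLevel.
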(event `RoundEnd`
  (bind _deadgoods (`self.DeadGoods`))
  (`/Engine/EditorBlueprintResources/ActorMacros.Switch Has Authority`
    (:`Authority`
      (for _array_element (`self.PlayerArray`)
        (bind _asbp_custom_player_state (cast `/Game/FirstPerson/Blueprints/BP_CustomPlayerState` _array_element))
        ;[1 1 1] True = Dead
        ; False = Alive
        (if (`/Game/FirstPerson/Blueprints/BP_CustomPlayerState.IsDead` _asbp_custom_player_state)
          (bind (_roledata_rolename _roledata_roleskeletal _roledata_rolestatic _roledata_rolematerial _roledata_isjoker_) (break `/Game/Meg/ST_RoleData` (`/Game/FirstPerson/Blueprints/BP_CustomPlayerState.RoleData` _asbp_custom_player_state)))
          (`KismetSystemLibrary.PrintString` (`KismetStringLibrary.Conv_BoolToString` _roledata_isjoker_) true true (struct :`R` 1.0 :`G` 0.510537 :`A` 1.0) 100.0)
          (if _roledata_isjoker_
            (`self.GoodWin`)
            (set `self.IsGameOver?` true)
            (else
              (`/Engine/EditorBlueprintResources/StandardMacros.IncrementInt` _deadgoods
                (:`  `
                  (if (== _deadgoods 3)
                    (`self.BadWin`)
                    (set `self.IsGameOver?` true))))))
          (else
            (`KismetSystemLibrary.PrintString` "Player Alive" true true (struct :`G` 1.0 :`B` 0.013185 :`A` 1.0) 5.0))))
      (if (not (`self.IsGameOver?`))
        (`self.NextRound`)))))

(event `GoodWin`
  ;[0 1 0.1571] Good Guys win
  (`KismetSystemLibrary.ExecuteConsoleCommand` "servertravel Lobby2" null))

(event `NextRound`
  ;[0 0.7937 1] Game still on
  (set `self.DeadGoods` 0)
  (`KismetSystemLibrary.ExecuteConsoleCommand` "servertravel MazeLevel" null))

(event `BadWin`
  ;[1 0.1036 0.1335] Joker Wins
  (`KismetSystemLibrary.ExecuteConsoleCommand` "servertravel Lobby2" null))

(fn `UserConstructionScript`)