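; Health component that tracks an actor's health and handles its death.
; ApplyDamage and ApplyHealth truncate amounts to integers and adjust Health; healing checks MaxHealth only before adding, so it can overshoot.
; At zero or below, DestroyOwner invokes CallDeath, destroying the owner and its pawn only when the owner is a PlayerState.
; Reset and max-health getter/setter functions are empty stubs, and debug prints remain.
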(event `/Game/Jacko/BPI_Health.ApplyDamage`
  (params (Damage :type "Float (double-precision)"))
  (`self.HealthDecrease` (`KismetMathLibrary.FTrunc` Damage)))

(event `/Game/Jacko/BPI_Health.ApplyHealth`
  (params (Healing :type "Float (double-precision)"))
  (`KismetSystemLibrary.PrintString` "sending to component")
  (`self.HealthIncrease` (`KismetMathLibrary.FTrunc` Healing)))

(event `DestroyOwner`
  (bind _returnvalue (`self.GetOwner`))
  (bind _asplayer_state (cast `PlayerState` _returnvalue)
    (:`then`
      (`self.Death`)
      (`Actor.K2_DestroyActor` _returnvalue)
      (`Actor.K2_DestroyActor` (`PlayerState.GetPawn` _asplayer_state)))
    (:`CastFailed`
      (`self.Death`))))

(fn `GetMaxHealth`)

(fn `HealthDecrease`
  (params (Damage :type Integer))
  (set `self.Health` (- (`self.Health`) Damage))
  (if (<= (`self.Health`) 0)
    (`self.DestroyOwner`)
    (`KismetSystemLibrary.PrintString` "Bruh dead" true true (struct :`R` 1.0 :`B` 0.496902 :`A` 1.0) 5.0)))

(fn `HealthIncrease`
  (params (Healing :type Integer))
  (if (>= (`self.Health`) (`self.MaxHealth`))
    (set `self.Health` (`self.MaxHealth`))
    (else
      (set `self.Health` (+ Healing (`self.Health`))))))

(fn `Reset Health`)

(fn `SetMaxHealth`)