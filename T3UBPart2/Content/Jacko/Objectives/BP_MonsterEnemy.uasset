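; BP_MonsterEnemy is an enemy that picks a random weakness, turns toward the player and destroys itself on health death.
; After a delay it creates a stacked-card widget and stores a random DataTable enemy's skeletal mesh and animation, but the OnRep code applying them is disconnected.
; FacePlayer loops through a tiny Delay.
; Sphere overlap switches health and card widgets between screen and world space, while VisibleVulnerability shows cards by health multiplier.
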(event `self.ReceiveBeginPlay`
  (bind _asbp_first_person_character (cast `/Game/FirstPerson/Blueprints/BP_FirstPersonCharacter` (`GameplayStatics.GetPlayerCharacter` 0)))
  (set `self.As BP First Person Character` _asbp_first_person_character)
  (`self.FacePlayer`)
  (bind _output_get (set `self.Weakness` (`KismetArrayLibrary.Array_Random` (`self.All weaknesses`))))
  (`KismetSystemLibrary.PrintString` (`KismetStringLibrary.Concat_StrStr` "Enemy weakness is" (`|GetEnumeratorNameAsString` _output_get)))
  (`KismetSystemLibrary.Delay` 5.0)
  (bind _returnvalue (`|CreateWidget` "/Game/Meg/Widgets/UMG_StackedCards.UMG_StackedCards_C"))
  (set `self.StackedCardWidget` _returnvalue)
  ;[1 1 1] Comment
  (`self.SetEnemy`))

(event `SetEnemy`
  ;[1 0.2077 0.5807] Sets Enemy meshes randomly
  (bind _outrownames (`DataTableFunctionLibrary.GetDataTableRowNames` "/Game/Jacko/Objectives/DT-EnemyTypes.DT-EnemyTypes"))
  (bind _returnvalue (`|GetDataTableRow` "/Game/Jacko/Objectives/DT-EnemyTypes.DT-EnemyTypes" (`KismetArrayLibrary.Array_Random` _outrownames))
    (:`then`
      (`self.UpdateEnemy` (break `/Game/Jacko/Objectives/ST_EnemyTypes` _returnvalue) (`.StaticMesh_5_A29C172A454C0DBC5A9B69919A57F76D` (break `/Game/Jacko/Objectives/ST_EnemyTypes` _returnvalue)) (`.SkeletalMesh_8_A750D3BC40093BE16396E88C239F95A3` (break `/Game/Jacko/Objectives/ST_EnemyTypes` _returnvalue)) (`.AnimationBlueprint_11_B63AD3BA4E8F8BB5EA0A16B08495EEE3` (break `/Game/Jacko/Objectives/ST_EnemyTypes` _returnvalue)))
      (`KismetSystemLibrary.PrintString` (break `/Game/Jacko/Objectives/ST_EnemyTypes` _returnvalue)))))

(event `self.BP_Health1.Death`
  (set `self.Dead?` true)
  (`self.MeDie`))

(event `UpdateEnemy`
  (params (EnemyName :type String) (enemyStaticMesh :type "StaticMesh Object Reference") (EnemySkeletalMesh :type "SkeletalMesh Object Reference") (AnimationBlueprint :type "AnimBlueprint Object Reference"))
  ;[1 0.2077 0.5807] Sets Enemy meshes randomly
  (set `self.Enemy Skeletal Mesh` EnemySkeletalMesh)
  (set `self.Animation Blueprint` AnimationBlueprint))

(event `MeDie`
  (`self.K2_DestroyActor`))

(event `FacePlayer`
  (bind (_returnvalue_roll _returnvalue_pitch _returnvalue_yaw) (`KismetMathLibrary.BreakRotator` (`KismetMathLibrary.RInterpTo` (`self.K2_GetActorRotation`) (`KismetMathLibrary.FindLookAtRotation` (`self.K2_GetActorLocation`) (`self.K2_GetActorLocation` (`self.As BP First Person Character`))) (`GameplayStatics.GetWorldDeltaSeconds`) 20.0)))
  (`self.K2_SetActorRotation` self (`KismetMathLibrary.MakeRotator` _returnvalue_roll _returnvalue_pitch _returnvalue_yaw) false)
  (`KismetSystemLibrary.Delay` 0.001)
  (`self.FacePlayer`))

(event `self.Sphere.OnComponentBeginOverlap`
  (params (OverlappedComponent :type "PrimitiveComponent Object Reference") (OtherActor :type "Actor Object Reference") (OtherComp :type "PrimitiveComponent Object Reference") (OtherBodyIndex :type Integer) (bFromSweep :type Boolean) (SweepResult :type "HitResult Structure (by ref)"))
  (`WidgetComponent.SetWidgetSpace` (`self.HealthBar`) "Screen")
  (`WidgetComponent.SetWidgetSpace` (`self.StackedCards`) "Screen"))

(event `self.Sphere.OnComponentEndOverlap`
  (params (OverlappedComponent :type "PrimitiveComponent Object Reference") (OtherActor :type "Actor Object Reference") (OtherComp :type "PrimitiveComponent Object Reference") (OtherBodyIndex :type Integer))
  (`WidgetComponent.SetWidgetSpace` (`self.HealthBar`) "World")
  (`WidgetComponent.SetWidgetSpace` (`self.StackedCards`) "World"))

(event `VisibleVulnerability`
  (bind _stackedcardwidget (`self.StackedCardWidget`))
  (bind _multiplier (`/Game/Jacko/BP_HealthComponent.Multiplier` (`self.BP_Health1`)))
  (bind _multiplier_2 (`/Game/Jacko/BP_HealthComponent.Multiplier` (`self.BP_Health1`)))
  ;[0.9878 0.1653 1] HandlesVisual Cards
  (`|ExecutionSequence`
    (:`then_0`
      (if (and (> _multiplier 0) (< _multiplier 2))
        (`Widget.SetVisibility` (`/Game/Meg/Widgets/UMG_StackedCards.LeftBox` (`self.StackedCardWidget`)) "Visible")))
    (:`then_1`
      (if (and (> _multiplier_2 1) (< _multiplier_2 3))
        (`Widget.SetVisibility` (`/Game/Meg/Widgets/UMG_StackedCards.MiddleBox` (`self.StackedCardWidget`)) "Visible")))
    (:`then_2`
      (if (> (`/Game/Jacko/BP_HealthComponent.Multiplier` (`self.BP_Health1`)) 2)
        (`Widget.SetVisibility` (`/Game/Meg/Widgets/UMG_StackedCards.RightBox` (`self.StackedCardWidget`)) "Visible")))
    (:`then_3`
      (if (<= (`/Game/Jacko/BP_HealthComponent.Multiplier` (`self.BP_Health1`)) 0)
        (`Widget.SetVisibility` (`/Game/Meg/Widgets/UMG_StackedCards.LeftBox` _stackedcardwidget) "SelfHitTestInvisible")
        (`Widget.SetVisibility` (`/Game/Meg/Widgets/UMG_StackedCards.RightBox` _stackedcardwidget) "SelfHitTestInvisible")
        (`Widget.SetVisibility` (`/Game/Meg/Widgets/UMG_StackedCards.MiddleBox` _stackedcardwidget) "SelfHitTestInvisible")))))

(fn `OnRep_Animation Blueprint`)

(fn `OnRep_Enemy Skeletal Mesh`)

(fn `UserConstructionScript`)