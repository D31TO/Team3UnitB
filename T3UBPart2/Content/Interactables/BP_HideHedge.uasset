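; BP_HideHedge is an interactable hedge that marks where the first-person player character can hide.
; On overlap with BP_FirstPersonCharacter it enables CanHide, sets the character's HideRef to itself and adds a WBP_BushPrompt widget to the viewport.
; When the overlap ends it disables CanHide and removes the prompt, leaving HideRef set.
; Both events print debug strings, and the hiding action itself is not handled here.
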(event `self.ReceiveActorBeginOverlap`
  (params (OtherActor :type "Actor Object Reference"))
  (bind _asbp_first_person_character (cast `/Game/FirstPerson/Blueprints/BP_FirstPersonCharacter` OtherActor))
  (set `/Game/FirstPerson/Blueprints/BP_FirstPersonCharacter.CanHide` true _asbp_first_person_character)
  (set `/Game/FirstPerson/Blueprints/BP_FirstPersonCharacter.HideRef` self _asbp_first_person_character)
  (`KismetSystemLibrary.PrintString` "Can hide" true true (struct :`G` 1.0 :`B` 0.181906 :`A` 1.0))
  (bind _returnvalue (`|CreateWidget` "/Game/Widgets/HUD/WBP_BushPrompt.WBP_BushPrompt_C"))
  (`UserWidget.AddToViewport` _returnvalue 0))

(event `self.ReceiveActorEndOverlap`
  (params (OtherActor :type "Actor Object Reference"))
  (bind _asbp_first_person_character (cast `/Game/FirstPerson/Blueprints/BP_FirstPersonCharacter` OtherActor))
  (set `/Game/FirstPerson/Blueprints/BP_FirstPersonCharacter.CanHide` false _asbp_first_person_character)
  (`KismetSystemLibrary.PrintString` "CANT HIDE" true true (struct :`R` 1.0 :`B` 0.086574 :`A` 1.0))
  (`Widget.RemoveFromParent` (stale `self.ReceiveActorBeginOverlap` _returnvalue)))

(fn `UserConstructionScript`)