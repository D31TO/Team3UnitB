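; Origami bat Blueprint that makes its skeletal mesh hover by bobbing up and down.
; BeginPlay reads the mesh's relative Z as a baseline, and Tick adds a degree-based sine of time since creation, scaled by BobbingSpeed and BobbingDistance.
; Each tick sets the whole relative transform with only Z supplied, leaving the other components at pin defaults.
; FacePlayer and the construction script are empty.
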(event `self.ReceiveBeginPlay`
  (set `self.Return Value Location Z` (.z (.location (`SceneComponent.GetRelativeTransform` (`self.SkeletalMesh`))))))

(event `self.ReceiveTick`
  (params (DeltaSeconds :type "Float (single-precision)"))
  (`SceneComponent.K2_SetRelativeTransform` (`self.SkeletalMesh`) (`KismetMathLibrary.MakeTransform` (`KismetMathLibrary.MakeVector` 0.0 0.0 (+ (* (`KismetMathLibrary.DegSin` (* (`self.GetGameTimeSinceCreation`) (`self.BobbingSpeed`))) (`self.bobbingDistance`)) (`self.Return Value Location Z`)))) false false))

(fn `FacePlayer`)

(fn `UserConstructionScript`)